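; Player-controlled boat that moves through physics forces on its BoatMesh.
; Move Forward and Move Right axis inputs apply acceleration-change forces along the actor's forward and right vectors, with weaker sideways push.
; Each Tick eases yaw toward the velocity direction with a fixed-alpha rotator lerp, keeping current pitch and roll, so steering follows movement and the smoothing depends on frame rate.
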(event `self.ReceiveBeginPlay`)

(event `InputAxis|Move Forward`
  (params (AxisValue :type "Float (single-precision)"))
  (`PrimitiveComponent.AddForce` (`self.BoatMesh`) (* (`self.GetActorForwardVector`) (* AxisValue 500.0)) "None" true))

(event `InputAxis|Move Right`
  (params (AxisValue :type "Float (single-precision)"))
  (`PrimitiveComponent.AddForce` (`self.BoatMesh`) (* (`self.GetActorRightVector`) (* AxisValue 300.0)) "None" true))

(event `self.ReceiveTick`
  (params (DeltaSeconds :type "Float (single-precision)"))
  (bind _returnvalue (`self.K2_GetActorRotation`))
  (bind (_returnvalue_roll _returnvalue_pitch _returnvalue_yaw) (`KismetMathLibrary.BreakRotator` (`KismetMathLibrary.RLerp` _returnvalue (`KismetMathLibrary.Conv_VectorToRotator` (`self.GetVelocity`)) 0.1)))
  (`self.K2_SetActorRotation` (`KismetMathLibrary.MakeRotator` (.roll _returnvalue) (.pitch _returnvalue) _returnvalue_yaw)))

(fn `UserConstructionScript`)